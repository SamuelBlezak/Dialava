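; BP_CraftingActor is a world crafting station that shows the crafting UI while something is within its collision sphere.
; Sphere begin and end overlaps, with no filter on the overlapping actor, call ToggleCrafting, guarded by the widget's validity.
; ToggleCrafting creates Wb_CraftingView and adds it to the viewport, or removes it and clears the reference.
; LookAt returns a "Použi {Name}" prompt, while the Interactwith event is empty.
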(event `self.SphereCollision.OnComponentEndOverlap`
  (params (OverlappedComponent :type "PrimitiveComponent Object Reference") (OtherActor :type "Actor Object Reference") (OtherComp :type "PrimitiveComponent Object Reference") (OtherBodyIndex :type Integer))
  (`self.CraftingViewWidget`
    (:`then`
      (`self.ToggleCrafting`))
    (:`else`)))

(event `/Game/Dialava/Interaction/BP_Interaction.InteractWith`
  (params (Interactor :type "Actor Object Reference")))

(event `self.SphereCollision.OnComponentBeginOverlap`
  (params (OverlappedComponent :type "PrimitiveComponent Object Reference") (OtherActor :type "Actor Object Reference") (OtherComp :type "PrimitiveComponent Object Reference") (OtherBodyIndex :type Integer) (bFromSweep :type Boolean) (SweepResult :type "HitResult Structure (by ref)"))
  (`self.CraftingViewWidget`
    (:`then`)
    (:`else`
      (`self.ToggleCrafting`))))

(fn `LookAt`
  (returns (HoverText :type Text))
  (return (`|FormatText` "Použi {Name}" (`self.Name`))))

(fn `ToggleCrafting`
  (bind _craftingviewwidget (`self.CraftingViewWidget`)
    (:`then`
      (`Widget.RemoveFromParent` _craftingviewwidget)
      (set `self.CraftingViewWidget` null))
    (:`else`
      (bind _returnvalue (`|CreateWidget` "/Game/Dialava/CraftingUI/Wb_CraftingView.Wb_CraftingView_C"))
      (bind _output_get (set `self.CraftingViewWidget` _returnvalue))
      (`UserWidget.AddToViewport` _output_get 0))))

(fn `UserConstructionScript`)