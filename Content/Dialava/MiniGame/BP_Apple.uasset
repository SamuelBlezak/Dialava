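; BP_Apple is a colored apple pickup for a minigame puzzle that the player submits by pressing E.
; A sphere overlap with BP_BaseCharacter enables input and interaction, and leaving the sphere disables both.
; On E it prints a debug message and passes its color to the referenced puzzle manager's CheckApple.
; The construction script sets the mesh material from the MyColor enum.
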(event `self.Sphere.OnComponentBeginOverlap`
  (params (OverlappedComponent :type "PrimitiveComponent Object Reference") (OtherActor :type "Actor Object Reference") (OtherComp :type "PrimitiveComponent Object Reference") (OtherBodyIndex :type Integer) (bFromSweep :type Boolean) (SweepResult :type "HitResult Structure (by ref)"))
  (cast `/Game/Dialava/Blueprints/BP_BaseCharacter` OtherActor)
  (set `self.CanInteract` true)
  (`self.EnableInput` (`GameplayStatics.GetPlayerController` 0)))

(event `self.Sphere.OnComponentEndOverlap`
  (params (OverlappedComponent :type "PrimitiveComponent Object Reference") (OtherActor :type "Actor Object Reference") (OtherComp :type "PrimitiveComponent Object Reference") (OtherBodyIndex :type Integer))
  (cast `/Game/Dialava/Blueprints/BP_BaseCharacter` OtherActor)
  (set `self.CanInteract` false)
  (`self.DisableInput` (`GameplayStatics.GetPlayerController` 0)))

(event `Key|E`
  (params (Key :type "Key Structure"))
  (:`Pressed`
    (if (`self.CanInteract`)
      (`KismetSystemLibrary.PrintString` "Hello")
      (`/Game/Dialava/MiniGame/BP_PuzzleManager.CheckApple` (`self.PuzzleManagerRef`) (`self.MyColor`)))))

(fn `UserConstructionScript`
  (`PrimitiveComponent.SetMaterial` (`self.tgzoahbpa_tier_3`) 0 (select `/Game/Dialava/MiniGame/E_Jablka` (`self.MyColor`) :`NewEnumerator0` "/Game/Fab/Megascans/3D/Red_Apple_tgzoahbpa/Low/MI_tgzoahbpa.MI_tgzoahbpa" :`NewEnumerator1` "/Game/Dialava/MiniGame/M_Green.M_Green" :`NewEnumerator2` "/Game/Dialava/MiniGame/M_Yellow.M_Yellow" :`NewEnumerator3` "/Game/Dialava/MiniGame/M_Blue.M_Blue" :!type "MaterialInterface Object Reference")))