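; BP_Radio is an interactable radio that plays music and advances two quest steps.
; An overlap box enables player input and shows the WB_Radio widget while the player character is inside.
; E cycles through the Playlist stations on the Hudba audio component, and F toggles it on or off.
; Each key also advances the game instance quest when its index is 8 or 9 respectively, before the CanInteract check.
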(event `self.Box.OnComponentBeginOverlap`
  (params (OverlappedComponent :type "PrimitiveComponent Object Reference") (OtherActor :type "Actor Object Reference") (OtherComp :type "PrimitiveComponent Object Reference") (OtherBodyIndex :type Integer) (bFromSweep :type Boolean) (SweepResult :type "HitResult Structure (by ref)"))
  (cast `/Game/Dialava/Blueprints/BP_BaseCharacter` OtherActor)
  (set `self.CanInteract` true)
  (`self.EnableInput` (`GameplayStatics.GetPlayerController` 0))
  (bind _returnvalue (`|CreateWidget` "/Game/Dialava/Widgets/WB_Radio.WB_Radio_C"))
  (`UserWidget.AddToViewport` _returnvalue 0))

(event `self.Box.OnComponentEndOverlap`
  (params (OverlappedComponent :type "PrimitiveComponent Object Reference") (OtherActor :type "Actor Object Reference") (OtherComp :type "PrimitiveComponent Object Reference") (OtherBodyIndex :type Integer))
  (cast `/Game/Dialava/Blueprints/BP_BaseCharacter` OtherActor)
  (set `self.CanInteract` false)
  (`self.DisableInput` (`GameplayStatics.GetPlayerController` 0))
  (`/Engine/EditorBlueprintResources/StandardMacros.IsValid` (stale `self.Box.OnComponentBeginOverlap` _returnvalue)
    (:`Is Valid`
      (`Widget.RemoveFromParent` (stale `self.Box.OnComponentBeginOverlap` _returnvalue)))))

(event `Key|E`
  (params (Key :type "Key Structure"))
  (bind _playlist (`self.Playlist`))
  (bind _hudba (`self.Hudba`))
  ;[1 1 1] prepinanie stanic
  (:`Pressed`
    (bind _asbp_game_instance (cast `/Game/Dialava/Blueprints/BP_GameInstance` (`GameplayStatics.GetGameInstance`)))
    (if (== (`/Game/Dialava/Blueprints/BP_GameInstance.CurrentQuestIndex` _asbp_game_instance) 8)
      (`/Game/Dialava/Blueprints/BP_GameInstance.AdvanceQuest` _asbp_game_instance))
    (if (`self.CanInteract`)
      (bind _result (`/Engine/EditorBlueprintResources/StandardMacros.IncrementInt` (`self.CurrentStationIndex`))
        (:`  `
          (bind _output_get (set `self.CurrentStationIndex` (mod _result (`KismetArrayLibrary.Array_Length` _playlist))))
          (`AudioComponent.SetSound` _hudba (`|GetArrayItem` _playlist _output_get))
          (`AudioComponent.Play` _hudba 0.0))))))

(event `Key|F`
  (params (Key :type "Key Structure"))
  (bind _hudba (`self.Hudba`))
  ;[1 1 1] vypnutie radia
  (:`Pressed`
    (bind _asbp_game_instance (cast `/Game/Dialava/Blueprints/BP_GameInstance` (`GameplayStatics.GetGameInstance`)))
    (if (== (`/Game/Dialava/Blueprints/BP_GameInstance.CurrentQuestIndex` _asbp_game_instance) 9)
      (`/Game/Dialava/Blueprints/BP_GameInstance.AdvanceQuest` _asbp_game_instance))
    (if (`self.CanInteract`)
      (if (not (`ActorComponent.IsActive` _hudba))
        (`ActorComponent.Activate` _hudba false)
        (else
          (`ActorComponent.Deactivate` _hudba))))))

(fn `UserConstructionScript`)