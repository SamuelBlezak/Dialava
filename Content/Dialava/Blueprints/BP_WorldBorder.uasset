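; BP_WorldBorder is a level boundary actor that warns the player and then moves them to another level.
; Entering the WarningBox with a BP_BaseCharacter sets a warning flag and shows a WB_GoBack widget, which is removed on exit.
; Any overlap with the TeleportBox plays a sound, waits briefly, then opens the level named by the Destination enum converted to a name.
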(event `self.WarningBox.OnComponentBeginOverlap`
  (params (OverlappedComponent :type "PrimitiveComponent Object Reference") (OtherActor :type "Actor Object Reference") (OtherComp :type "PrimitiveComponent Object Reference") (OtherBodyIndex :type Integer) (bFromSweep :type Boolean) (SweepResult :type "HitResult Structure (by ref)"))
  (cast `/Game/Dialava/Blueprints/BP_BaseCharacter` OtherActor)
  (set `self.insideWarning` true)
  (bind _returnvalue (`|CreateWidget` "/Game/Dialava/Widgets/WB_GoBack.WB_GoBack_C"))
  (`UserWidget.AddToViewport` _returnvalue 0))

(event `self.WarningBox.OnComponentEndOverlap`
  (params (OverlappedComponent :type "PrimitiveComponent Object Reference") (OtherActor :type "Actor Object Reference") (OtherComp :type "PrimitiveComponent Object Reference") (OtherBodyIndex :type Integer))
  (cast `/Game/Dialava/Blueprints/BP_BaseCharacter` OtherActor)
  (set `self.insideWarning` false)
  (`Widget.RemoveFromParent` (stale `self.WarningBox.OnComponentBeginOverlap` _returnvalue)))

(event `self.TeleportBox.OnComponentBeginOverlap`
  (params (OverlappedComponent :type "PrimitiveComponent Object Reference") (OtherActor :type "Actor Object Reference") (OtherComp :type "PrimitiveComponent Object Reference") (OtherBodyIndex :type Integer) (bFromSweep :type Boolean) (SweepResult :type "HitResult Structure (by ref)"))
  (`GameplayStatics.PlaySound2D` "/Game/Dialava/Sounds/fahhh_KcgAXfs.fahhh_KcgAXfs" 1.0 1.0 0.0 null null)
  (`KismetSystemLibrary.Delay` 1.0)
  (`GameplayStatics.OpenLevel` (`KismetStringLibrary.Conv_StringToName` (`|GetEnumeratorNameAsString` (`self.Destination`)))))

(fn `UserConstructionScript`)