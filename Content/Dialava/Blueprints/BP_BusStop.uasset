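; Bus stop trigger that ends this part of the game when the player reaches it at a specific quest stage.
; On character overlap at that stage, it advances the quest, clears widgets, enters cinematic mode and plays the LS_Ending sequence.
; After a fixed delay, it copies survival stats, money, monologue progress and inventory into the GameInstance to persist them, then opens the Mesto level.
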(event `self.Box.OnComponentBeginOverlap`
  (params (OverlappedComponent :type "PrimitiveComponent Object Reference") (OtherActor :type "Actor Object Reference") (OtherComp :type "PrimitiveComponent Object Reference") (OtherBodyIndex :type Integer) (bFromSweep :type Boolean) (SweepResult :type "HitResult Structure (by ref)"))
  (bind _returnvalue (`GameplayStatics.GetPlayerCharacter` 0))
  (bind _asbp_base_character (cast `/Game/Dialava/Blueprints/BP_BaseCharacter` OtherActor))
  (bind _asbp_game_instance (cast `/Game/Dialava/Blueprints/BP_GameInstance` (`GameplayStatics.GetGameInstance`)))
  (if (== (`/Game/Dialava/Blueprints/BP_GameInstance.CurrentQuestIndex` _asbp_game_instance) 12)
    (bind _asbp_game_instance_2 (cast `/Game/Dialava/Blueprints/BP_GameInstance` (`GameplayStatics.GetGameInstance`)))
    (`/Game/Dialava/Blueprints/BP_GameInstance.AdvanceQuest` _asbp_game_instance_2)
    (`WidgetLayoutLibrary.RemoveAllWidgets`)
    (`PlayerController.SetCinematicMode` (`PlayerState.GetPlayerController` (`Pawn.PlayerState` _asbp_base_character)) true true true true true)
    (bind (_outactor _returnvalue_2) (`LevelSequencePlayer.CreateLevelSequencePlayer` "/Game/Dialava/Cutscenes/LS_Ending.LS_Ending"))
    (`MovieSceneSequencePlayer.Play` _returnvalue_2)
    (`KismetSystemLibrary.Delay` 10.0)
    (bind _asbp_base_character_2 (cast `/Game/Dialava/Blueprints/BP_BaseCharacter` _returnvalue))
    (bind _asbp_game_instance_3 (cast `/Game/Dialava/Blueprints/BP_GameInstance` (`GameplayStatics.GetGameInstance`)))
    (set `/Game/Dialava/Blueprints/BP_GameInstance.Water` (`/Game/Dialava/Blueprints/BP_BaseCharacter.CurrentWater` _asbp_base_character_2) _asbp_game_instance_3)
    (set `/Game/Dialava/Blueprints/BP_GameInstance.Food` (`/Game/Dialava/Blueprints/BP_BaseCharacter.CurrentFood` _asbp_base_character_2) _asbp_game_instance_3)
    (set `/Game/Dialava/Blueprints/BP_GameInstance.Money` (`/Game/Dialava/Blueprints/BP_BaseCharacter.CurrentMoney` _asbp_base_character_2) _asbp_game_instance_3)
    (set `/Game/Dialava/Blueprints/BP_GameInstance.MonologueIndex` (`/Game/Dialava/Blueprints/BP_BaseCharacter.MonologueIndex` _asbp_base_character_2) _asbp_game_instance_3)
    (set `/Game/Dialava/Blueprints/BP_GameInstance.Inventory` (`/Game/Dialava/Inventory/BPC_Inventory.ItemSlots` (`self.GetComponentByClass` _returnvalue "/Game/Dialava/Inventory/BPC_Inventory.BPC_Inventory_C")) _asbp_game_instance_3)
    (`GameplayStatics.OpenLevel` "Mesto")))

(fn `UserConstructionScript`)