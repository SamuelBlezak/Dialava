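; BP_BabkaNPC is an NPC Blueprint that steps through a dialogue on screen with voice playback.
; Each Talk event advances Index and shows that Dialogue line in a WB_Dialogue widget, created when none exists.
; It stops the previous voice and spawns the Voice sound at its owner's location.
; Once the lines run out, Talk removes the widget without resetting Index.
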(event `/Game/Dialava/Blueprints/BPI_Dialogue.Talk`
  (bind _currentvoice (`self.CurrentVoice`))
  (`/Engine/EditorBlueprintResources/StandardMacros.IncrementInt` (`self.Index`)
    (:`  `
      (if (< (`self.Index`) (`KismetArrayLibrary.Array_Length` (`self.Dialogue`)))
        (`self.WB_Dialogue`
          (:`then`
            _)
          (:`else`
            (bind _returnvalue (`|CreateWidget` "/Game/Dialava/Blueprints/WB_Dialogue.WB_Dialogue_C" (`GameplayStatics.GetPlayerController` 0)))
            (bind _output_get (set `self.WB_Dialogue` _returnvalue))
            (`UserWidget.AddToViewport` _output_get 0)))
        (`TextBlock.SetText` (`/Game/Dialava/Blueprints/WB_Dialogue.DialogueText` (`self.WB_Dialogue`)) (`KismetTextLibrary.Conv_StringToText` (`|GetArrayItem` (`self.Dialogue`) (`self.Index`))))
        (bind _voice (`self.Voice`)
          (:`then`
            (`/Engine/EditorBlueprintResources/StandardMacros.IsValid` _currentvoice
              (:`Is Valid`
                (`AudioComponent.Stop` _currentvoice))
              (:`Is Not Valid`
                _)))
          (:`else`
            _))
        (bind _returnvalue_2 (`GameplayStatics.SpawnSoundAtLocation` _voice (`self.K2_GetActorLocation` (`self.GetOwner`)) (struct) 1.0 1.0 0.0 null null))
        (bind _output_get_2 (set `self.CurrentVoice` _returnvalue_2))
        (`AudioComponent.Play` _output_get_2 1.0)
        (else
          (`Widget.RemoveFromParent` (`self.WB_Dialogue`)))))))

(fn `UserConstructionScript`)