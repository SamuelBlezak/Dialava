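; Daylight blueprint that advances a day cycle by rotating a referenced sun light and adjusting its brightness.
; PassTime pitches the sun in local space in proportion to the passed time, then feeds its up-vector Z as sun height into ChangeLightIntensity.
; That height is remapped and clamped over a narrow band around zero to blend between dim and bright intensity.
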(fn `PassTime_0`
  (params (PassedTime :type "Float (double-precision)") (SunReference :type "DirectionalLight Object Reference"))
  (bind (_returnvalue_x _returnvalue_y _returnvalue_z) (`KismetMathLibrary.BreakVector` (`Actor.GetActorUpVector` SunReference)))
  (`self.MoveSun` PassedTime SunReference)
  (`self.ChangeLightIntensity` SunReference _returnvalue_z))