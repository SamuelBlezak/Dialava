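; BP_Flask is a quest pickup actor that a BP_BaseCharacter collects by overlapping its Box during quest index 8.
; Collection advances the quest in BP_GameInstance, plays a pickup sound at the world origin, sets FlaskCollected and destroys the actor.
; On BeginPlay it reads that same game instance flag and destroys itself if the flask was already collected.
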(event `self.ReceiveBeginPlay`
  (bind _asbp_game_instance (cast `/Game/Dialava/Blueprints/BP_GameInstance` (`GameplayStatics.GetGameInstance`)))
  (if (`/Game/Dialava/Blueprints/BP_GameInstance.FlaskCollected` _asbp_game_instance)
    (`self.K2_DestroyActor`)))

(event `self.Box.OnComponentBeginOverlap`
  (params (OverlappedComponent :type "PrimitiveComponent Object Reference") (OtherActor :type "Actor Object Reference") (OtherComp :type "PrimitiveComponent Object Reference") (OtherBodyIndex :type Integer) (bFromSweep :type Boolean) (SweepResult :type "HitResult Structure (by ref)"))
  (cast `/Game/Dialava/Blueprints/BP_BaseCharacter` OtherActor)
  (bind _asbp_game_instance (cast `/Game/Dialava/Blueprints/BP_GameInstance` (`GameplayStatics.GetGameInstance`)))
  (if (== (`/Game/Dialava/Blueprints/BP_GameInstance.CurrentQuestIndex` _asbp_game_instance) 8)
    (`/Game/Dialava/Blueprints/BP_GameInstance.AdvanceQuest` _asbp_game_instance)
    (`GameplayStatics.PlaySoundAtLocation` "/Game/Dialava/Sounds/gta-pick-up.gta-pick-up" (0.0 0.0 0.0) (struct) 1.0 1.0 0.0 null null null null)
    (bind _asbp_game_instance_2 (cast `/Game/Dialava/Blueprints/BP_GameInstance` (`GameplayStatics.GetGameInstance`)))
    (set `/Game/Dialava/Blueprints/BP_GameInstance.FlaskCollected` true _asbp_game_instance_2)
    (`self.K2_DestroyActor`)))

(fn `UserConstructionScript`)