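; BP_Button is an interactable trigger actor that activates a boost on the player's character.
; When a BP_BaseCharacter enters its Box, it allows interaction, enables input and shows a WB_Button widget; leaving reverses this.
; Releasing E while interaction is allowed sets IsBoostActive on the character, reusing the actor reference from the overlap event.
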(event `self.Box.OnComponentBeginOverlap`
  (params (OverlappedComponent :type "PrimitiveComponent Object Reference") (OtherActor :type "Actor Object Reference") (OtherComp :type "PrimitiveComponent Object Reference") (OtherBodyIndex :type Integer) (bFromSweep :type Boolean) (SweepResult :type "HitResult Structure (by ref)"))
  (cast `/Game/Dialava/Blueprints/BP_BaseCharacter` OtherActor)
  (set `self.CanInteract` true)
  (`self.EnableInput` (`GameplayStatics.GetPlayerController` 0))
  (bind _returnvalue (`|CreateWidget` "/Game/Dialava/Widgets/WB_Button.WB_Button_C"))
  (`UserWidget.AddToViewport` _returnvalue 0))

(event `self.Box.OnComponentEndOverlap`
  (params (OverlappedComponent :type "PrimitiveComponent Object Reference") (OtherActor :type "Actor Object Reference") (OtherComp :type "PrimitiveComponent Object Reference") (OtherBodyIndex :type Integer))
  (cast `/Game/Dialava/Blueprints/BP_BaseCharacter` OtherActor)
  (set `self.CanInteract` false)
  (`self.DisableInput` (`GameplayStatics.GetPlayerController` 0))
  (`/Engine/EditorBlueprintResources/StandardMacros.IsValid` (stale `self.Box.OnComponentBeginOverlap` _returnvalue)
    (:`Is Valid`
      (`Widget.RemoveFromParent` (stale `self.Box.OnComponentBeginOverlap` _returnvalue)))))

(event `Key|E`
  (params (Key :type "Key Structure"))
  (:`Released`
    (if (`self.CanInteract`)
      (bind _asbp_base_character (cast `/Game/Dialava/Blueprints/BP_BaseCharacter` (stale `self.Box.OnComponentEndOverlap` OtherActor)))
      (set `/Game/Dialava/Blueprints/BP_BaseCharacter.IsBoostActive` true _asbp_base_character))))

(fn `UserConstructionScript`)