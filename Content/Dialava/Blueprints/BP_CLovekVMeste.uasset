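; BP_CLovekVMeste is a wandering town NPC that the player can pickpocket.
; It roams to random nearby points, and when PawnSensing spots a non-crouching player it plays a debounced sound and flees directly away.
; Its overlap sphere shows a BP_Skillcheck widget while the player is in range.
; UkradniPeniaze (steal money) transfers its money to the thief and advances the quest if index 18 is active.
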(event `self.ReceiveTick`
  (params (DeltaSeconds :type "Float (single-precision)"))
  (if (not (`self.IsSeeingPlayer?`))
    (`KismetSystemLibrary.Delay` (`KismetMathLibrary.RandomFloatInRange` 2.0 5.0))
    (set `self.IsMoving?` true)
    (`|AIMoveTo` self (`NavigationSystemV1.K2_GetRandomReachablePointInRadius` (`self.K2_GetActorLocation`) 500.0 null null) null
      (:`OnSuccess`
        (set `self.IsMoving?` false)))))

(event `self.PawnSensing.OnSeePawn`
  (params (Pawn :type "Pawn Object Reference"))
  (bind _returnvalue (`self.K2_GetActorLocation`))
  (bind _asbp_base_character (cast `/Game/Dialava/Blueprints/BP_BaseCharacter` Pawn))
  (if (not (`/Game/Dialava/Blueprints/BP_BaseCharacter.IsCrouching` _asbp_base_character))
    (`|ExecutionSequence`
      (:`then_0`
        (`|ExecutionSequence`
          (:`then_0`
            (`/Engine/EditorBlueprintResources/StandardMacros.DoOnce` false :!label _label
              (:`Completed`
                (`GameplayStatics.PlaySoundAtLocation` "/Game/Dialava/Sounds/fahhh_KcgAXfs.fahhh_KcgAXfs" (`self.K2_GetActorLocation`) (struct) 1.0 0.5 0.0 null null null null))))
          (:`then_1`
            (`KismetSystemLibrary.RetriggerableDelay` 2.0)
            (goto _label :!via `Reset`))))
      (:`then_1`
        (`|ExecutionSequence`
          (:`then_0`
            (set `self.IsSeeingPlayer?` true)
            (set `self.IsMoving?` true)
            (`|AIMoveTo` self (`KismetMathLibrary.MakeVector` (.x (+ _returnvalue (* (`KismetMathLibrary.GetForwardVector` (`KismetMathLibrary.FindLookAtRotation` _returnvalue (`self.K2_GetActorLocation` _asbp_base_character))) -500.0))) (.y (+ _returnvalue (* (`KismetMathLibrary.GetForwardVector` (`KismetMathLibrary.FindLookAtRotation` _returnvalue (`self.K2_GetActorLocation` _asbp_base_character))) -500.0))) (.z _returnvalue)) null))
          (:`then_1`
            (`KismetSystemLibrary.Delay` 0.5)
            (set `self.IsSeeingPlayer?` false)))))))

(event `self.Sphere.OnComponentBeginOverlap`
  (params (OverlappedComponent :type "PrimitiveComponent Object Reference") (OtherActor :type "Actor Object Reference") (OtherComp :type "PrimitiveComponent Object Reference") (OtherBodyIndex :type Integer) (bFromSweep :type Boolean) (SweepResult :type "HitResult Structure (by ref)"))
  (bind _asbp_base_character (cast `/Game/Dialava/Blueprints/BP_BaseCharacter` OtherActor))
  (set `self.CanInteract` true)
  (bind _returnvalue (`|CreateWidget` "/Game/Dialava/Widgets/BP_Skillcheck.BP_Skillcheck_C" null _asbp_base_character))
  (bind _output_get (set `self.NewVar` _returnvalue))
  (`UserWidget.AddToViewport` _output_get 0))

(event `self.Sphere.OnComponentEndOverlap`
  (params (OverlappedComponent :type "PrimitiveComponent Object Reference") (OtherActor :type "Actor Object Reference") (OtherComp :type "PrimitiveComponent Object Reference") (OtherBodyIndex :type Integer))
  (cast `/Game/Dialava/Blueprints/BP_BaseCharacter` OtherActor)
  (set `self.CanInteract` false)
  (`Widget.RemoveFromParent` (`self.NewVar`))
  (set `self.NewVar` null))

(event `UkradniPeniaze`
  (params (Thief :type "/Game/Dialava/Blueprints/BP_BaseCharacter Object Reference"))
  (set `/Game/Dialava/Blueprints/BP_BaseCharacter.CurrentMoney` (+ (`/Game/Dialava/Blueprints/BP_BaseCharacter.CurrentMoney` Thief) (`self.Peniaze`)) Thief)
  (set `self.Peniaze` 0)
  (bind _asbp_game_instance (cast `/Game/Dialava/Blueprints/BP_GameInstance` (`GameplayStatics.GetGameInstance`)))
  (if (== (`/Game/Dialava/Blueprints/BP_GameInstance.CurrentQuestIndex` _asbp_game_instance) 18)
    (`/Game/Dialava/Blueprints/BP_GameInstance.AdvanceQuest` _asbp_game_instance)))

(fn `UserConstructionScript`)