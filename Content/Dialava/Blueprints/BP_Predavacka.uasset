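; BP_Predavacka is a shopkeeper NPC that charges the player for eggs and flour carried in their inventory.
; Each Talk call recomputes the total from BPC_Inventory counts, selecting default dialogue or a price line and advancing the quest from step 2 if there is a charge.
; Repeated calls step through WB_Dialogue text with pitched voice audio, then close it and deduct the total from BP_BaseCharacter's money.
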(event `self.Talk`
  (bind _currentvoice (`self.CurrentVoice`))
  (bind _returnvalue (`self.GetComponentByClass` (`GameplayStatics.GetPlayerCharacter` 0) "/Game/Dialava/Inventory/BPC_Inventory.BPC_Inventory_C"))
  (set `self.Suma` 0)
  (set `self.Talking` true)
  (bind (_pocet _success) (`/Game/Dialava/Inventory/BPC_Inventory.CheckInventory` _returnvalue "Vajcia_001"))
  (if _success
    (set `self.Suma` (+ (`self.Suma`) (* _pocet 2))))
  (bind (_pocet_2 _success_2) (`/Game/Dialava/Inventory/BPC_Inventory.CheckInventory` _returnvalue "Muka_001"))
  (if _success_2
    (set `self.Suma` (+ (`self.Suma`) (* _pocet_2 3))))
  (if (== (`self.Suma`) 0)
    (set `self.CoSaPovie` (`self.Dialogue_0`))
    (else
      (bind _output_get (set `self.VetaSoSumou` (`KismetStringLibrary.Concat_StrStr` "Bude to stáť " (`KismetStringLibrary.Conv_IntToString` (`self.Suma`)) " eur")))
      (set `self.Dialogue_1` (`|MakeArray` _output_get))
      (set `self.CoSaPovie` (`self.Dialogue_1`))
      (bind _asbp_game_instance (cast `/Game/Dialava/Blueprints/BP_GameInstance` (`GameplayStatics.GetGameInstance`)))
      (if (== (`/Game/Dialava/Blueprints/BP_GameInstance.CurrentQuestIndex` _asbp_game_instance) 2)
        (`/Game/Dialava/Blueprints/BP_GameInstance.AdvanceQuest` _asbp_game_instance))))
  (`/Engine/EditorBlueprintResources/StandardMacros.IncrementInt` (`self.Index`)
    (:`  `
      (if (< (`self.Index`) (`KismetArrayLibrary.Array_Length` (`self.CoSaPovie`)))
        (`self.WB_Dialogue`
          (:`then`
            _)
          (:`else`
            (bind _returnvalue_2 (`|CreateWidget` "/Game/Dialava/Blueprints/WB_Dialogue.WB_Dialogue_C" (`GameplayStatics.GetPlayerController` 0)))
            (bind _output_get_2 (set `self.WB_Dialogue` _returnvalue_2))
            (`UserWidget.AddToViewport` _output_get_2 0)))
        (`TextBlock.SetText` (`/Game/Dialava/Blueprints/WB_Dialogue.DialogueText` (`self.WB_Dialogue`)) (`KismetTextLibrary.Conv_StringToText` (`|GetArrayItem` (`self.CoSaPovie`) (`self.Index`))))
        (bind _voice (`self.Voice`)
          (:`then`
            (`/Engine/EditorBlueprintResources/StandardMacros.IsValid` _currentvoice
              (:`Is Valid`
                (`AudioComponent.Stop` _currentvoice))
              (:`Is Not Valid`
                _)))
          (:`else`
            _))
        (bind _returnvalue_3 (`GameplayStatics.SpawnSoundAtLocation` _voice (`self.K2_GetActorLocation` (`self.GetOwner`)) (struct) 1.2 1.3 0.0 null null))
        (bind _output_get_3 (set `self.CurrentVoice` _returnvalue_3))
        (`AudioComponent.Play` _output_get_3 1.0)
        (else
          (`Widget.RemoveFromParent` (`self.WB_Dialogue`))
          (set `self.Index` -1)
          (set `self.WB_Dialogue` null)
          (set `self.Talking` false)
          (bind _asbp_base_character (cast `/Game/Dialava/Blueprints/BP_BaseCharacter` (`GameplayStatics.GetPlayerCharacter` 0)))
          (set `/Game/Dialava/Blueprints/BP_BaseCharacter.CurrentMoney` (- (`/Game/Dialava/Blueprints/BP_BaseCharacter.CurrentMoney` _asbp_base_character) (`self.Suma`)) _asbp_base_character))))))

(fn `UserConstructionScript`)