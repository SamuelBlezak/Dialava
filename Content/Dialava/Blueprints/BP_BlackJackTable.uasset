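; Interactable blackjack table where the player bets money against a dealer.
; Entering its box shows a prompt; pressing E with enough money switches the camera and opens the game UI.
; It shuffles six decks, takes the stake, deals card widgets with one dealer card hidden, and scores aces as 11 or 1.
; The dealer turn recursively draws with a delay until 17 or higher, then wins pay double and ties refund.
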(event `self.Box.OnComponentBeginOverlap`
  (params (OverlappedComponent :type "PrimitiveComponent Object Reference") (OtherActor :type "Actor Object Reference") (OtherComp :type "PrimitiveComponent Object Reference") (OtherBodyIndex :type Integer) (bFromSweep :type Boolean) (SweepResult :type "HitResult Structure (by ref)"))
  (cast `/Game/Dialava/Blueprints/BP_BaseCharacter` OtherActor)
  (set `self.CanInteract` true)
  (`self.EnableInput` (`GameplayStatics.GetPlayerController` 0))
  (bind _returnvalue (`|CreateWidget` "/Game/Dialava/Widgets/WB_BlackJack.WB_BlackJack_C"))
  (`UserWidget.AddToViewport` _returnvalue 0))

(event `self.Box.OnComponentEndOverlap`
  (params (OverlappedComponent :type "PrimitiveComponent Object Reference") (OtherActor :type "Actor Object Reference") (OtherComp :type "PrimitiveComponent Object Reference") (OtherBodyIndex :type Integer))
  (cast `/Game/Dialava/Blueprints/BP_BaseCharacter` OtherActor)
  (set `self.CanInteract` false)
  (`self.DisableInput` (`GameplayStatics.GetPlayerController` 0))
  (`/Engine/EditorBlueprintResources/StandardMacros.IsValid` (stale `self.Box.OnComponentBeginOverlap` _returnvalue)
    (:`Is Valid`
      (`Widget.RemoveFromParent` (stale `self.Box.OnComponentBeginOverlap` _returnvalue)))))

(event `Key|E`
  (params (Key :type "Key Structure"))
  (bind _returnvalue (`GameplayStatics.GetPlayerController` 0))
  (:`Pressed`
    (bind _asbp_base_character (cast `/Game/Dialava/Blueprints/BP_BaseCharacter` (`GameplayStatics.GetPlayerCharacter` 0)))
    (set `self.PlayerRef` _asbp_base_character)
    (if (and (`self.CanInteract`) (>= (`/Game/Dialava/Blueprints/BP_BaseCharacter.CurrentMoney` (`self.PlayerRef`)) (`self.Stavka`)))
      (`Widget.RemoveFromParent` (stale `self.Box.OnComponentBeginOverlap` _returnvalue))
      (`PlayerController.SetViewTargetWithBlend` (`GameplayStatics.GetPlayerController` 0) self 0.5 "VTBlend_Linear" 0.0 false)
      (bind _returnvalue_2 (`|CreateWidget` "/Game/Dialava/Widgets/WB_BlackjackUI.WB_BlackjackUI_C" null self))
      (set `self.Ref_HlavneMenu` _returnvalue_2)
      (`UserWidget.AddToViewport` _returnvalue_2 0)
      (`WidgetBlueprintLibrary.SetInputMode_UIOnlyEx` _returnvalue _returnvalue_2)
      (set `PlayerController.bShowMouseCursor` true _returnvalue)
      (`self.GenerateDeck`)
      (`self.StartNewGame`))))

(event `PlayDealerTurn`
  (bind _finalscore (`self.CalculateScore` (`self.DealerHand`)))
  (if (< _finalscore 17)
    (`KismetSystemLibrary.Delay` 1.0)
    (`self.DrawCard` false)
    (`self.UpdateScores`)
    (`self.PlayDealerTurn`)
    (else
      (`self.CheckWinner`))))

(event `EndGame`
  (params (ResultMessage :type String))
  (`/Game/Dialava/Widgets/WB_BlackjackUI.ZobrazVysledok` (`self.Ref_HlavneMenu`) ResultMessage))

(fn `CalculateScore`
  (params (Hand :type "Array of /Game/Dialava/MiniGame/BlackjackMinigame/S_Card Structure"))
  (returns (FinalScore :type Integer))
  (locals (TempScore :type Integer) (AcesCount :type Integer))
  (set `local.AcesCount` 0)
  (set `local.TempScore` 0)
  (for _array_element Hand
    (bind (_suit _rank _value) (break `/Game/Dialava/MiniGame/BlackjackMinigame/S_Card` _array_element))
    (set `local.TempScore` (+ _value (`local.TempScore`)))
    (if (`|EnumEquality` _rank "NewEnumerator12")
      (bind _result (`/Engine/EditorBlueprintResources/StandardMacros.IncrementInt` (`local.AcesCount`))
        (:`  `
          (set `local.AcesCount` _result)))))
  (while (and (> (`local.TempScore`) 21) (> (`local.AcesCount`) 0))
    (set `local.TempScore` (- (`local.TempScore`) 10))
    (set `local.AcesCount` (- (`local.AcesCount`) 1)))
  (return (`local.TempScore`)))

(fn `CheckWinner`
  (locals (SkoreHrac :type Integer) (SkoreKrupier :type Integer))
  (bind _playerref (`self.PlayerRef`))
  (bind _playerref_2 (`self.PlayerRef`))
  (bind _returnvalue (+ (`/Game/Dialava/Blueprints/BP_BaseCharacter.CurrentMoney` _playerref) (* (`self.Stavka`) 2)))
  (bind _finalscore (`self.CalculateScore` (`self.PlayerHand`)))
  (set `local.SkoreHrac` _finalscore)
  (bind _finalscore_2 (`self.CalculateScore` (`self.DealerHand`)))
  (set `local.SkoreKrupier` _finalscore_2)
  (if (> (`local.SkoreKrupier`) 21)
    (set `/Game/Dialava/Blueprints/BP_BaseCharacter.CurrentMoney` _returnvalue _playerref)
    (`self.EndGame` "Krupiér prekročil 21. VYHRAL SI!")
    (elif (> (`local.SkoreHrac`) (`local.SkoreKrupier`))
      (set `/Game/Dialava/Blueprints/BP_BaseCharacter.CurrentMoney` _returnvalue _playerref)
      (`self.EndGame` "VYHRAL SI!")
      (elif (== (`local.SkoreHrac`) (`local.SkoreKrupier`))
        (set `/Game/Dialava/Blueprints/BP_BaseCharacter.CurrentMoney` (+ (`/Game/Dialava/Blueprints/BP_BaseCharacter.CurrentMoney` _playerref_2) (`self.Stavka`)) _playerref_2)
        (`self.EndGame` "REMÍZA (Push)")
        (else
          (`self.EndGame` "PREHRAL SI!"))))))

(fn `DrawCard`
  (params (IsPlayer :type Boolean) (FaceDown :type Boolean))
  (locals (DrawnCard :type "/Game/Dialava/MiniGame/BlackjackMinigame/S_Card Structure"))
  (bind _drawncard (`local.DrawnCard`))
  (set `local.DrawnCard` (`|GetArrayItem` (`self.Deck`)))
  (`KismetArrayLibrary.Array_Remove` (`self.Deck`))
  (if IsPlayer
    (`KismetArrayLibrary.Array_Add` (`self.PlayerHand`) _drawncard)
    (else
      (`KismetArrayLibrary.Array_Add` (`self.DealerHand`) _drawncard)))
  (bind _returnvalue (`|CreateWidget` "/Game/Dialava/MiniGame/BlackjackMinigame/WB_Card.WB_Card_C" null _drawncard FaceDown))
  (if IsPlayer
    (bind _returnvalue_2 (`HorizontalBox.AddChildToHorizontalBox` (`/Game/Dialava/Widgets/WB_BlackjackUI.HBox_PlayerCards` (`self.Ref_HlavneMenu`)) _returnvalue))
    (`HorizontalBoxSlot.SetPadding` _returnvalue_2 (make `Margin` 70.0))
    (else
      (bind _returnvalue_3 (`HorizontalBox.AddChildToHorizontalBox` (`/Game/Dialava/Widgets/WB_BlackjackUI.HBox_DealerCards` (`self.Ref_HlavneMenu`)) _returnvalue))
      (`HorizontalBoxSlot.SetPadding` _returnvalue_3 (make `Margin` 70.0))))
  (`self.UpdateScores`)
  (bind _finalscore (`self.CalculateScore` (`self.PlayerHand`)))
  (if (and (`local.IsPlayer`) (> _finalscore 21))
    (`self.EndGame` "BUST! Prekročil si 21.")))

(fn `GenerateDeck`
  (`KismetArrayLibrary.Array_Clear` (`self.Deck`))
  (for _ (range 1 7)
    (for _index (range 4)
      (for _index_2 (range 13)
        (bind _returnvalue (cast `/Game/Dialava/MiniGame/BlackjackMinigame/E_CardRank` (`KismetMathLibrary.Conv_IntToByte` _index_2)))
        (`KismetArrayLibrary.Array_Add` (`self.Deck`) (make `/Game/Dialava/MiniGame/BlackjackMinigame/S_Card` (cast `/Game/Dialava/MiniGame/BlackjackMinigame/E_CardSuit` (`KismetMathLibrary.Conv_IntToByte` _index)) _returnvalue (select `/Game/Dialava/MiniGame/BlackjackMinigame/E_CardRank` _returnvalue :`NewEnumerator0` 2 :`NewEnumerator1` 3 :`NewEnumerator2` 4 :`NewEnumerator3` 5 :`NewEnumerator4` 6 :`NewEnumerator5` 7 :`NewEnumerator6` 8 :`NewEnumerator7` 9 :`NewEnumerator8` 10 :`NewEnumerator9` 10 :`NewEnumerator10` 10 :`NewEnumerator11` 10 :`NewEnumerator12` 11))))))
  (`KismetArrayLibrary.Array_Shuffle` (`self.Deck`)))

(fn `StartNewGame`
  (locals (NewLocalVar :type "/Game/Dialava/Widgets/WB_BlackjackUI Object Reference"))
  (bind _playerref (`self.PlayerRef`))
  (bind _stavka (`self.Stavka`))
  (bind _currentmoney (`/Game/Dialava/Blueprints/BP_BaseCharacter.CurrentMoney` _playerref))
  (if (>= _currentmoney _stavka)
    (set `/Game/Dialava/Blueprints/BP_BaseCharacter.CurrentMoney` (- _currentmoney _stavka) _playerref)
    (set `self.bIsDealerCardHidden` true)
    (`KismetArrayLibrary.Array_Clear` (`self.PlayerHand`))
    (`KismetArrayLibrary.Array_Clear` (`self.DealerHand`))
    (`PanelWidget.ClearChildren` (`/Game/Dialava/Widgets/WB_BlackjackUI.HBox_PlayerCards` (`self.Ref_HlavneMenu`)))
    (`PanelWidget.ClearChildren` (`/Game/Dialava/Widgets/WB_BlackjackUI.HBox_DealerCards` (`self.Ref_HlavneMenu`)))
    (`self.DrawCard` true)
    (`self.DrawCard` false)
    (`self.DrawCard` true)
    (`self.DrawCard` false true)
    (`self.UpdateScores`)))

(fn `UpdateScores`
  (bind (_output_suit _output_rank _output_value) (break `/Game/Dialava/MiniGame/BlackjackMinigame/S_Card` (`|GetArrayItem` (`self.DealerHand`))))
  (bind _finalscore (`self.CalculateScore` (`self.PlayerHand`)))
  (`TextBlock.SetText` (`/Game/Dialava/Widgets/WB_BlackjackUI.Txt_PlayerScore` (`self.Ref_HlavneMenu`)) (`KismetTextLibrary.Conv_StringToText` (`KismetStringLibrary.Concat_StrStr` "Skóre: " (`KismetStringLibrary.Conv_IntToString` _finalscore))))
  (if (`self.bIsDealerCardHidden`)
    (`TextBlock.SetText` (`/Game/Dialava/Widgets/WB_BlackjackUI.Txt_DealerScore` (`self.Ref_HlavneMenu`)) (`KismetTextLibrary.Conv_StringToText` (`KismetStringLibrary.Concat_StrStr` "Skóre: " (`KismetStringLibrary.Conv_IntToString` _output_value))))
    (else
      (bind _finalscore_2 (`self.CalculateScore` (`self.DealerHand`)))
      (`TextBlock.SetText` (`/Game/Dialava/Widgets/WB_BlackjackUI.Txt_DealerScore` (`self.Ref_HlavneMenu`)) (`KismetTextLibrary.Conv_StringToText` (`KismetStringLibrary.Concat_StrStr` "Skóre: " (`KismetStringLibrary.Conv_IntToString` _finalscore_2)))))))

(fn `UserConstructionScript`)