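; Daylight helper functions that run a day-night cycle on a sun light actor passed in by reference.
; PassTime pitches the sun by elapsed time times a speed, which is ten times faster while its forward vector points upward (night).
; It then sets light intensity by a clamped lerp on the Z of the sun's up vector, blending between dim and bright around zero.
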(fn `ChangeLightIntensity`
  (params (SunHeight :type "Float (double-precision)") (SunReference :type "DirectionalLight Object Reference"))
  (`LightComponent.SetIntensity` (`Light.LightComponent` SunReference) (`KismetMathLibrary.Lerp` 0.5 10.0 (`KismetMathLibrary.FClamp` (/ (+ SunHeight 0.2) 0.4)))))

(fn `GetSunSpeedFromDaytime`
  (params (SunReference :type "DirectionalLight Object Reference"))
  (returns (SunSpeed :type "Float (double-precision)"))
  (bind (_returnvalue_x _returnvalue_y _returnvalue_z) (`KismetMathLibrary.BreakVector` (`Actor.GetActorForwardVector` SunReference)))
  (if (> _returnvalue_z 0.0)
    (return 10.0)
    (else
      (return 1.0))))

(fn `MoveSun`
  (params (PassedTime :type "Float (double-precision)") (SunReference :type "DirectionalLight Object Reference") (SunSpeed :type "Float (double-precision)"))
  (`Actor.K2_AddActorLocalRotation` SunReference (`KismetMathLibrary.MakeRotator` 0.0 (* PassedTime SunSpeed)) false false))

(fn `PassTime`
  (params (PassedTime :type "Float (double-precision)") (SunReference :type "DirectionalLight Object Reference"))
  (bind (_returnvalue_x _returnvalue_y _returnvalue_z) (`KismetMathLibrary.BreakVector` (`Actor.GetActorUpVector` SunReference)))
  (bind _sunspeed (`self.GetSunSpeedFromDaytime` SunReference))
  (`self.MoveSun` PassedTime SunReference _sunspeed)
  (`self.ChangeLightIntensity` _returnvalue_z SunReference))