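; Player character for Dialava, handling movement, sprint boost, pause menu, quest log and F-key NPC dialogue through BPI_Dialogue.
; Once the intro flag is set, BeginPlay loads stats from BP_GameInstance, creates HUD, minimap and quest log, and starts random sounds.
; Looping timers drain food and water, then money; Tick pauses and shows the death screen when money turns negative.
; Intro cutscene, inventory toggle and crouch capsule resize are disconnected.
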(event `EnhancedInput|/Game/Inputs/IA_Look`
  (params (ActionValue :type "Vector2D Structure") (ElapsedSeconds :type "Float (double-precision)") (TriggeredSeconds :type "Float (double-precision)") (InputAction :type "InputAction Object Reference" :default "/Game/Inputs/IA_Look.IA_Look"))
  (:`Triggered`
    (`self.AddControllerYawInput` ActionValue_X)
    (`self.AddControllerPitchInput` ActionValue_Y)))

(event `EnhancedInput|/Game/Inputs/IA_MoveForward`
  (params (ActionValue :type "Float (double-precision)") (ElapsedSeconds :type "Float (double-precision)") (TriggeredSeconds :type "Float (double-precision)") (InputAction :type "InputAction Object Reference" :default "/Game/Inputs/IA_MoveForward.IA_MoveForward"))
  (bind (_returnvalue_roll _returnvalue_pitch _returnvalue_yaw) (`KismetMathLibrary.BreakRotator` (`self.GetControlRotation`)))
  (:`Triggered`
    (bind _output_get (set `self.Forward` ActionValue))
    (`self.AddMovementInput` (`KismetMathLibrary.GetForwardVector` (`KismetMathLibrary.MakeRotator` 0.0 0.0 _returnvalue_yaw)) _output_get)
    (set `self.IsWalking` true))
  (:`Canceled`
    (set `self.IsWalking` false :!label _label)
    (set `self.Forward` 0.0))
  (:`Completed`
    (goto _label)))

(event `EnhancedInput|/Game/Inputs/IA_MoveRight`
  (params (ActionValue :type "Float (double-precision)") (ElapsedSeconds :type "Float (double-precision)") (TriggeredSeconds :type "Float (double-precision)") (InputAction :type "InputAction Object Reference" :default "/Game/Inputs/IA_MoveRight.IA_MoveRight"))
  (bind (_returnvalue_roll _returnvalue_pitch _returnvalue_yaw) (`KismetMathLibrary.BreakRotator` (`self.GetControlRotation`)))
  (:`Triggered`
    (bind _output_get (set `self.Right` ActionValue))
    (`self.AddMovementInput` (`KismetMathLibrary.GetRightVector` (`KismetMathLibrary.MakeRotator` 0.0 0.0 _returnvalue_yaw)) _output_get)
    (set `self.IsWalking` true))
  (:`Canceled`
    (set `self.IsWalking` false :!label _label_2)
    (set `self.Right` 0.0))
  (:`Completed`
    (goto _label_2)))

(event `EnhancedInput|/Game/Inputs/IA_Sprint`
  (params (ActionValue :type Boolean) (ElapsedSeconds :type "Float (double-precision)") (TriggeredSeconds :type "Float (double-precision)") (InputAction :type "InputAction Object Reference" :default "/Game/Inputs/IA_Sprint.IA_Sprint"))
  (bind _charactermovement (`self.CharacterMovement`))
  (:`Triggered`
    (if (`self.IsBoostActive`)
      (set `CharacterMovementComponent.MaxWalkSpeed` 6000.0 _charactermovement)
      (`KismetSystemLibrary.Delay` 15.0)
      (set `self.IsBoostActive` false))
    (set `CharacterMovementComponent.MaxWalkSpeed` 1200.0 _charactermovement)
    (set `self.IsRunning` true))
  (:`Canceled`
    (set `CharacterMovementComponent.MaxWalkSpeed` 600.0 _charactermovement :!label _label_3)
    (set `self.IsRunning` false))
  (:`Completed`
    (goto _label_3)))

(event `EnhancedInput|/Game/Inputs/IA_Jump`
  (params (ActionValue :type Boolean) (ElapsedSeconds :type "Float (double-precision)") (TriggeredSeconds :type "Float (double-precision)") (InputAction :type "InputAction Object Reference" :default "/Game/Inputs/IA_Jump.IA_Jump"))
  (:`Triggered`
    (if (not (`self.IsJumping`))
      (`self.Jump`)
      (`self.Jump`)))
  (:`Canceled`
    (`self.StopJumping` :!label _label_4))
  (:`Completed`
    (goto _label_4)))

(event `self.OnJumped`
  (set `self.IsJumping` true))

(event `self.OnLanded`
  (params (Hit :type "HitResult Structure (by ref)"))
  (`KismetSystemLibrary.Delay` 0.4)
  (set `self.IsJumping` false))

(event `EnhancedInput|/Game/Inputs/IA_Crouch`
  (params (ActionValue :type Boolean) (ElapsedSeconds :type "Float (double-precision)") (TriggeredSeconds :type "Float (double-precision)") (InputAction :type "InputAction Object Reference" :default "/Game/Inputs/IA_Crouch.IA_Crouch"))
  (bind _charactermovement (`self.CharacterMovement`))
  (:`Triggered`
    (set `self.IsCrouching` true)
    (set `CharacterMovementComponent.MaxWalkSpeed` 300.0 _charactermovement))
  (:`Canceled`
    (set `self.IsCrouching` false :!label _label_5)
    (set `CharacterMovementComponent.MaxWalkSpeed` 600.0 _charactermovement))
  (:`Completed`
    (goto _label_5)))

(event `EnhancedInput|/Game/Inputs/IA_Pause`
  (params (ActionValue :type Boolean) (ElapsedSeconds :type "Float (double-precision)") (TriggeredSeconds :type "Float (double-precision)") (InputAction :type "InputAction Object Reference" :default "/Game/Inputs/IA_Pause.IA_Pause"))
  (bind _returnvalue (`GameplayStatics.GetPlayerController` 0))
  (:`Started`
    (if (not (`self.IsPauseMenuOpen`))
      (set `self.IsPauseMenuOpen` true)
      (bind _returnvalue_2 (`|CreateWidget` "/Game/Dialava/Blueprints/WB_PauseMenu.WB_PauseMenu_C" _returnvalue))
      (bind _output_get (set `self.PauseMenuWidget` _returnvalue_2))
      (`UserWidget.AddToViewport` _output_get 0)
      (`WidgetBlueprintLibrary.SetInputMode_GameAndUIEx` _returnvalue (`self.PauseMenuWidget`))
      (set `PlayerController.bShowMouseCursor` true (`GameplayStatics.GetPlayerController` 0))
      (`GameplayStatics.SetGamePaused` true)
      (else
        (set `self.IsPauseMenuOpen` false)
        (`Widget.RemoveFromParent` (`self.PauseMenuWidget`))
        (`GameplayStatics.SetGamePaused` false)
        (`WidgetBlueprintLibrary.SetInputMode_GameOnly` _returnvalue)
        (set `PlayerController.bShowMouseCursor` false (`GameplayStatics.GetPlayerController` 0))))))

(event `EnhancedInput|/Game/Inputs/IA_Inventory`
  (params (ActionValue :type Boolean) (ElapsedSeconds :type "Float (double-precision)") (TriggeredSeconds :type "Float (double-precision)") (InputAction :type "InputAction Object Reference" :default "/Game/Inputs/IA_Inventory.IA_Inventory")))

(event `self.ReceiveBeginPlay`
  (bind _asbp_game_instance (cast `/Game/Dialava/Blueprints/BP_GameInstance` (`GameplayStatics.GetGameInstance`)))
  (if (`/Game/Dialava/Blueprints/BP_GameInstance.IntroPlayed` _asbp_game_instance)
    (`self.DisplayPlayerHUD`)
    ;[1 1 1] loadovanie statov z game instance do current hodnot
    (bind _asbp_game_instance_2 (cast `/Game/Dialava/Blueprints/BP_GameInstance` (`GameplayStatics.GetGameInstance`)))
    (set `self.CurrentMoney` (`/Game/Dialava/Blueprints/BP_GameInstance.Money` _asbp_game_instance_2))
    (set `self.CurrentFood` (`/Game/Dialava/Blueprints/BP_GameInstance.Food` _asbp_game_instance_2))
    (set `self.CurrentWater` (`/Game/Dialava/Blueprints/BP_GameInstance.Water` _asbp_game_instance_2))
    (set `self.MonologueIndex` (`/Game/Dialava/Blueprints/BP_GameInstance.MonologueIndex` _asbp_game_instance_2))
    (bind _returnvalue (`|CreateWidget` "/Game/Dialava/Widgets/WB_Minimap.WB_Minimap_C" (`GameplayStatics.GetPlayerController` 0)))
    (`UserWidget.AddToViewport` _returnvalue 0)
    (bind _returnvalue_2 (`|CreateWidget` "/Game/Dialava/Widgets/WB_QuestLog.WB_QuestLog_C"))
    (set `self.QuestLogWidgetRef` _returnvalue_2)
    ;[1 1 1] DepleteStats
    (`KismetSystemLibrary.K2_SetTimerDelegate` (delegate `DepleteFood`) 5.0 true)
    (`KismetSystemLibrary.K2_SetTimerDelegate` (delegate `DepleteWater`) 3.0 true)
    (bind _asbp_game_instance_3 (cast `/Game/Dialava/Blueprints/BP_GameInstance` (`GameplayStatics.GetGameInstance`)))
    (set `SpringArmComponent.bDoCollisionTest` (`/Game/Dialava/Blueprints/BP_GameInstance.MinimapCollision` _asbp_game_instance_3) (`self.SpringArm1`))
    (`self.RandomNoise`)
    (else
      (set `/Game/Dialava/Blueprints/BP_GameInstance.IntroPlayed` true _asbp_game_instance)
      (`WidgetLayoutLibrary.RemoveAllWidgets`))))

(event `DepleteFood`
  ;[1 1 1] DepleteStats
  (if (> (`self.CurrentFood`) 0.0)
    (set `self.CurrentFood` (- (`self.CurrentFood`) 1.0))
    (else
      (set `self.CurrentMoney` (- (`self.CurrentMoney`) 2) :!label _label_6))))

(event `DepleteWater`
  ;[1 1 1] DepleteStats
  (if (> (`self.CurrentWater`) 0.0)
    (set `self.CurrentWater` (- (`self.CurrentWater`) 1.0))
    (else
      (goto _label_6))))

(event `EnhancedInput|/Game/Inputs/IA_OpenQuestLog`
  (params (ActionValue :type Boolean) (ElapsedSeconds :type "Float (double-precision)") (TriggeredSeconds :type "Float (double-precision)") (InputAction :type "InputAction Object Reference" :default "/Game/Inputs/IA_OpenQuestLog.IA_OpenQuestLog"))
  (bind _questlogwidgetref (`self.QuestLogWidgetRef`))
  (:`Started`
    (`/Engine/EditorBlueprintResources/StandardMacros.FlipFlop`
      (:`A`
        (`UserWidget.AddToViewport` _questlogwidgetref 0))
      (:`B`
        (`Widget.RemoveFromParent` _questlogwidgetref)))))

(event `Key|F`
  (params (Key :type "Key Structure"))
  (:`Pressed`
    (for _array_element (`self.GetOverlappingActors` "/Game/Dialava/Blueprints/BP_BabkaNPC.BP_BabkaNPC_C")
      (if (`KismetSystemLibrary.DoesImplementInterface` _array_element "/Game/Dialava/Blueprints/BPI_Dialogue.BPI_Dialogue_C")
        (message `/Game/Dialava/Blueprints/BPI_Dialogue.Talk` _array_element)))))

(event `Key|F`
  (params (Key :type "Key Structure"))
  (:`Pressed`
    (for _array_element (`self.GetOverlappingActors` "/Game/Dialava/Blueprints/BP_Ferenci.BP_Ferenci_C")
      (if (`KismetSystemLibrary.DoesImplementInterface` _array_element "/Game/Dialava/Blueprints/BPI_Dialogue.BPI_Dialogue_C")
        (message `/Game/Dialava/Blueprints/BPI_Dialogue.Talk` _array_element)))))

(event `Key|F`
  (params (Key :type "Key Structure"))
  (:`Pressed`
    (for _array_element (`self.GetOverlappingActors` "/Game/Dialava/Blueprints/BP_Predavacka.BP_Predavacka_C")
      (if (`KismetSystemLibrary.DoesImplementInterface` _array_element "/Game/Dialava/Blueprints/BPI_Dialogue.BPI_Dialogue_C")
        (message `/Game/Dialava/Blueprints/BPI_Dialogue.Talk` _array_element)))))

(event `SwitchMinimapCollision`
  (params (ShouldCollide :type Boolean))
  (set `SpringArmComponent.bDoCollisionTest` ShouldCollide (`self.SpringArm1`)))

(event `RandomNoise`
  (`KismetSystemLibrary.Delay` (`KismetMathLibrary.RandomFloatInRange` 30.0 120.0))
  (`GameplayStatics.PlaySound2D` "/Game/Dialava/Sounds/SoundCue/SC_CharacterSounds.SC_CharacterSounds" 1.0 1.0 0.0 null null)
  (`self.RandomNoise`))

(event `self.ReceiveTick`
  (params (DeltaSeconds :type "Float (single-precision)"))
  (if (< (`self.CurrentMoney`) 0)
    (`GameplayStatics.SetGamePaused` true)
    (`WidgetBlueprintLibrary.SetInputMode_GameOnly` (`GameplayStatics.GetPlayerController` 0))
    (set `PlayerController.bShowMouseCursor` true (`GameplayStatics.GetPlayerController` 0))
    (bind _returnvalue (`|CreateWidget` "/Game/Dialava/Blueprints/WB_Death.WB_Death_C"))
    (`UserWidget.AddToViewport` _returnvalue 0)))

(fn `DisplayInventoryUI`
  (bind _returnvalue (`self.GetComponentByClass` (`GameplayStatics.GetPlayerCharacter` 0) "/Game/Dialava/Inventory/BPC_Inventory.BPC_Inventory_C"))
  (`/Engine/EditorBlueprintResources/StandardMacros.IsValid` _returnvalue
    (:`Is Valid`
      (bind _returnvalue_2 (`|CreateWidget` "/Game/Dialava/Inventory/UI/WB_InventoryUI.WB_InventoryUI_C" null _returnvalue))
      (bind _output_get (set `self.WB_InventoryUI` _returnvalue_2))
      (`UserWidget.AddToViewport` _output_get 0))))

(fn `DisplayPlayerHUD`
  (bind _returnvalue (`|CreateWidget` "/Game/Dialava/Interaction/UI/WB_PlayerHUD.WB_PlayerHUD_C"))
  (bind _output_get (set `self.WB_PlayerHUD` _returnvalue))
  (`UserWidget.AddToViewport` _output_get 0))

(fn `UserConstructionScript`)