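; BP_MinesTable is an interactable table that opens the Mines minigame UI for the player.
; Box overlap with a BP_BaseCharacter enables input on the table and shows the WB_MinesPlay widget, and leaving reverses both.
; Pressing E in range blends the view to the table and opens WB_MinesMain with a reference back to it.
; The mouse cursor then appears and input switches to UI only.
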(event `self.Box.OnComponentBeginOverlap`
  (params (OverlappedComponent :type "PrimitiveComponent Object Reference") (OtherActor :type "Actor Object Reference") (OtherComp :type "PrimitiveComponent Object Reference") (OtherBodyIndex :type Integer) (bFromSweep :type Boolean) (SweepResult :type "HitResult Structure (by ref)"))
  (cast `/Game/Dialava/Blueprints/BP_BaseCharacter` OtherActor)
  (set `self.CanInteract` true)
  (`self.EnableInput` (`GameplayStatics.GetPlayerController` 0))
  (bind _returnvalue (`|CreateWidget` "/Game/Dialava/Widgets/WB_MinesPlay.WB_MinesPlay_C"))
  (`UserWidget.AddToViewport` _returnvalue 0))

(event `self.Box.OnComponentEndOverlap`
  (params (OverlappedComponent :type "PrimitiveComponent Object Reference") (OtherActor :type "Actor Object Reference") (OtherComp :type "PrimitiveComponent Object Reference") (OtherBodyIndex :type Integer))
  (cast `/Game/Dialava/Blueprints/BP_BaseCharacter` OtherActor)
  (set `self.CanInteract` false)
  (`self.DisableInput` (`GameplayStatics.GetPlayerController` 0))
  (`/Engine/EditorBlueprintResources/StandardMacros.IsValid` (stale `self.Box.OnComponentBeginOverlap` _returnvalue)
    (:`Is Valid`
      (`Widget.RemoveFromParent` (stale `self.Box.OnComponentBeginOverlap` _returnvalue)))))

(event `Key|E`
  (params (Key :type "Key Structure"))
  (bind _returnvalue (`GameplayStatics.GetPlayerController` 0))
  (:`Pressed`
    (if (`self.CanInteract`)
      (`PlayerController.SetViewTargetWithBlend` (`GameplayStatics.GetPlayerController` 0) self 0.5 "VTBlend_Linear" 0.0 false)
      (bind _returnvalue_2 (`|CreateWidget` "/Game/Dialava/MiniGame/MinesMinigame/WB_MinesMain.WB_MinesMain_C" null self))
      (bind _output_get (set `self.RefMinesUI` _returnvalue_2))
      (`UserWidget.AddToViewport` _output_get 0)
      (`WidgetBlueprintLibrary.SetInputMode_UIOnlyEx` _returnvalue null)
      (set `PlayerController.bShowMouseCursor` true _returnvalue))))

(fn `UserConstructionScript`)