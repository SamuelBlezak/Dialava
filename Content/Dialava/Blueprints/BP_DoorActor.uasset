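; BP_DoorActor is an interactable door that moves the player character to another level.
; Overlapping its box enables input and shows a "get inside" widget, both cleared on exit.
; Releasing E advances the quest if it is at index 1, saves water, food, money, inventory and door ID to BP_GameInstance, then opens the level named by the Destination enum.
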(event `self.Box.OnComponentBeginOverlap`
  (params (OverlappedComponent :type "PrimitiveComponent Object Reference") (OtherActor :type "Actor Object Reference") (OtherComp :type "PrimitiveComponent Object Reference") (OtherBodyIndex :type Integer) (bFromSweep :type Boolean) (SweepResult :type "HitResult Structure (by ref)"))
  ;[1 1 1] V boxe
  (cast `/Game/Dialava/Blueprints/BP_BaseCharacter` OtherActor)
  (set `self.CanInteract` true)
  (`self.EnableInput` (`GameplayStatics.GetPlayerController` 0))
  ;[1 1 1] Widget show/hide
  (bind _returnvalue (`|CreateWidget` "/Game/Dialava/Widgets/WB_GetInside.WB_GetInside_C"))
  (`UserWidget.AddToViewport` _returnvalue 0))

(event `self.Box.OnComponentEndOverlap`
  (params (OverlappedComponent :type "PrimitiveComponent Object Reference") (OtherActor :type "Actor Object Reference") (OtherComp :type "PrimitiveComponent Object Reference") (OtherBodyIndex :type Integer))
  ;[1 1 1] Mimo boxu
  (cast `/Game/Dialava/Blueprints/BP_BaseCharacter` OtherActor)
  (set `self.CanInteract` false)
  (`self.DisableInput` (`GameplayStatics.GetPlayerController` 0))
  ;[1 1 1] Widget show/hide
  (`/Engine/EditorBlueprintResources/StandardMacros.IsValid` (stale `self.Box.OnComponentBeginOverlap` _returnvalue)
    (:`Is Valid`
      (`Widget.RemoveFromParent` (stale `self.Box.OnComponentBeginOverlap` _returnvalue)))))

(event `Key|E`
  (params (Key :type "Key Structure"))
  (:`Released`
    (if (`self.CanInteract`)
      (bind _asbp_base_character (cast `/Game/Dialava/Blueprints/BP_BaseCharacter` (stale `self.Box.OnComponentBeginOverlap` OtherActor)))
      (bind _asbp_game_instance (cast `/Game/Dialava/Blueprints/BP_GameInstance` (`GameplayStatics.GetGameInstance`)))
      (if (== (`/Game/Dialava/Blueprints/BP_GameInstance.CurrentQuestIndex` _asbp_game_instance) 1)
        (`/Game/Dialava/Blueprints/BP_GameInstance.AdvanceQuest` _asbp_game_instance))
      (set `/Game/Dialava/Blueprints/BP_GameInstance.Water` (`/Game/Dialava/Blueprints/BP_BaseCharacter.CurrentWater` _asbp_base_character) _asbp_game_instance)
      (set `/Game/Dialava/Blueprints/BP_GameInstance.Food` (`/Game/Dialava/Blueprints/BP_BaseCharacter.CurrentFood` _asbp_base_character) _asbp_game_instance)
      (set `/Game/Dialava/Blueprints/BP_GameInstance.Money` (`/Game/Dialava/Blueprints/BP_BaseCharacter.CurrentMoney` _asbp_base_character) _asbp_game_instance)
      (set `/Game/Dialava/Blueprints/BP_GameInstance.Inventory` (`/Game/Dialava/Inventory/BPC_Inventory.ItemSlots` (`self.GetComponentByClass` (`GameplayStatics.GetPlayerCharacter` 0) "/Game/Dialava/Inventory/BPC_Inventory.BPC_Inventory_C")) _asbp_game_instance)
      ;[1 1 1] otvorenie levelu
      (set `/Game/Dialava/Blueprints/BP_GameInstance.DoorID` (`self.DoorID`) _asbp_game_instance)
      (`GameplayStatics.OpenLevel` (`KismetStringLibrary.Conv_StringToName` (`|GetEnumeratorNameAsString` (`self.Destination`)))))))

(fn `UserConstructionScript`)