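; BP_BaseMode is a game mode that picks the player's spawn point from the door ID stored in the game instance.
; Its FindPlayerStart override returns the first PlayerStart whose tag equals BP_GameInstance's DoorID, falling back to the first one found.
; The incoming start name is ignored, and the search runs only if the game instance casts to BP_GameInstance.
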(fn `FindPlayerStart`
  (params (Player :type "Controller Object Reference") (IncomingName :type String))
  (returns (ReturnValue :type "Actor Object Reference"))
  (bind _asbp_game_instance (cast `/Game/Dialava/Blueprints/BP_GameInstance` (`GameplayStatics.GetGameInstance`)))
  (bind _outactors (`GameplayStatics.GetAllActorsOfClass` "/Script/Engine.PlayerStart"))
  (for _array_element _outactors
    (if (== (`PlayerStart.PlayerStartTag` _array_element) (`/Game/Dialava/Blueprints/BP_GameInstance.DoorID` _asbp_game_instance))
      (return _array_element)))
  (return (`|GetArrayItem` _outactors)))

(fn `UserConstructionScript`)