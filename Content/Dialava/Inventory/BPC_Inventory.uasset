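; Inventory component that stores items in a fixed-size slot array, using DT_ItemData for stack limits, actor classes and sounds.
; PickUp adds one unit to a matching non-full stack or the first empty slot.
; Dropping spawns the item in a random cone ahead of the owner.
; UseItem consumes three hardcoded food and water items to raise BP_BaseCharacter stats, and changes are broadcast through OnInventoryUpdated.
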(event `self.ReceiveBeginPlay`
  (`KismetArrayLibrary.Array_Resize` (`self.ItemSlots`) (`self.InventorySize`)))

(event `UpdateInventory`
  (`self.OnInventoryUpdated`))

(fn `AddToMatchingSlot`
  (params (Index :type Integer) (ItemQuantity :type Integer))
  (bind (_itemid _itemquantity) (break `/Game/Dialava/Inventory/ItemData/S_ItemSlot` (`|GetArrayItem` (`self.ItemSlots`) Index)))
  (`KismetArrayLibrary.Array_Set` (`self.ItemSlots`) (`local.Index`) (make `/Game/Dialava/Inventory/ItemData/S_ItemSlot` _itemid (+ _itemquantity ItemQuantity))))

(fn `AddToNewSlot`
  (params (ItemID :type Name) (ItemQuantity :type Integer) (Index :type Integer))
  (`KismetArrayLibrary.Array_Set` (`self.ItemSlots`) Index (make `/Game/Dialava/Inventory/ItemData/S_ItemSlot` ItemID ItemQuantity)))

(fn `AnyAvailableSlots`
  (returns (Success :type Boolean) (Index :type Integer))
  (for (_array_element _array_index) (`self.ItemSlots`)
    (if (== (`.ItemQuantity_5_66F1C66E4ADE1E87F04247ADE9BF1AF0` (break `/Game/Dialava/Inventory/ItemData/S_ItemSlot` _array_element)) 0)
      (return true _array_index)))
  (return false -1))

(fn `DropFromInventory`
  (params (ItemID :type Name) (ItemQuantity :type Integer) (Index :type Integer))
  (bind _returnvalue (- ItemQuantity 1))
  (`|SpawnActorFromClass` (`.ItemClass_14_FEC3E33240D84B2F5FA349B7085A97D6` (break `/Game/Dialava/Inventory/ItemData/S_ItemInfo` (`self.GetItemData` ItemID))) (`KismetMathLibrary.MakeTransform` (`self.GetDropLocation`)) "Undefined" "MultiplyWithRoot" null null)
  (if (> _returnvalue 0)
    (`KismetArrayLibrary.Array_Set` (`self.ItemSlots`) (`local.Index`) (make `/Game/Dialava/Inventory/ItemData/S_ItemSlot` (`local.ItemID`) _returnvalue))
    (else
      (`KismetArrayLibrary.Array_Set` (`self.ItemSlots`) (`local.Index`) (make `/Game/Dialava/Inventory/ItemData/S_ItemSlot` "None"))))
  (`self.UpdateInventory`)
  (`self.PlaySoundEffect` (`.PickUp_4_8E67154F42B05F19198E6089657685A6` (break `/Game/Dialava/Inventory/ItemData/S_ItemSoundEffects` (`self.GetItemSoundEffect` (`local.ItemID`))))))

(fn `FindMatchingSlot`
  (params (ItemdID :type Name))
  (returns (Index :type Integer) (Success :type Boolean))
  (for (_array_element _array_index) (`self.ItemSlots`)
    (bind (_itemid _itemquantity) (break `/Game/Dialava/Inventory/ItemData/S_ItemSlot` _array_element))
    (if (and (== _itemid (`local.ItemdID`)) (< _itemquantity (`.SlotQuantity_17_B084497D4947A4EB54705086583A60B6` (break `/Game/Dialava/Inventory/ItemData/S_ItemInfo` (`self.GetItemData` (`local.ItemdID`))))))
      (return _array_index true)))
  (return -1 false))

(fn `GetDropLocation`
  (returns (DropLocation :type "Vector Structure"))
  (bind _returnvalue (`self.GetOwner`))
  (return (+ (`Actor.K2_GetActorLocation` _returnvalue) (* (`KismetMathLibrary.RandomUnitVectorInConeInDegrees` (`Actor.GetActorForwardVector` _returnvalue) 55.0) 100.0))))

(fn `GetItemData`
  (params (RowID :type Name))
  (returns (ItemData :type "/Game/Dialava/Inventory/ItemData/S_ItemInfo Structure"))
  (bind _returnvalue (`|GetDataTableRow` "/Game/Dialava/Inventory/ItemData/DT_ItemData.DT_ItemData" RowID)
    (:`then`
      (return _returnvalue))))

(fn `GetItemSoundEffect`
  (params (ItemID :type Name))
  (returns (ItemSoundEffects :type "/Game/Dialava/Inventory/ItemData/S_ItemSoundEffects Structure"))
  (return (`.ItemSoundEffects_15_C9590D0D4935B10B4127458B4DFE0731` (break `/Game/Dialava/Inventory/ItemData/S_ItemInfo` (`self.GetItemData` ItemID)))))

(fn `PickUp`
  (params (ItemID :type Name) (ItemQuantity :type Integer))
  (returns (Success :type Boolean) (ItemQuantityLeft :type Integer))
  (locals (Local_ItemQuantity :type Integer) (LocalIsFull :type Boolean :default false))
  (bind (_success _index) (`self.AnyAvailableSlots`))
  (bind _output_get (set `local.Local_ItemQuantity` ItemQuantity))
  (while (and (> _output_get 0) (not (`local.LocalIsFull`)))
    (bind (_index_2 _success_2) (`self.FindMatchingSlot` (`local.ItemID`)))
    (if _success_2
      (`self.AddToMatchingSlot` _index_2 1)
      (`/Engine/EditorBlueprintResources/StandardMacros.DecrementInt` (`local.Local_ItemQuantity`) :!label _label
        (:`  `
          (`self.PlaySoundEffect` (`.PickUp_4_8E67154F42B05F19198E6089657685A6` (break `/Game/Dialava/Inventory/ItemData/S_ItemSoundEffects` (`self.GetItemSoundEffect` (`local.ItemID`)))))
          (`self.UpdateInventory`)
          (return true 0)))
      (elif _success
        (`self.AddToNewSlot` (`local.ItemID`) 1 _index)
        (goto _label))))
  (`self.UpdateInventory`)
  (return (not (`local.LocalIsFull`)) (`local.Local_ItemQuantity`)))

(fn `PlaySoundEffect`
  (params (Sound :type "SoundBase Object Reference"))
  (`GameplayStatics.PlaySoundAtLocation` Sound (`Actor.K2_GetActorLocation` (`self.GetOwner`)) (struct) 1.0 1.0 0.0 null null null null))

(fn `PrintInventory`
  (for (_array_element _array_index) (`self.ItemSlots`)
    (bind (_itemid _itemquantity) (break `/Game/Dialava/Inventory/ItemData/S_ItemSlot` _array_element))
    (`KismetSystemLibrary.PrintString` (`KismetStringLibrary.Concat_StrStr` (`KismetStringLibrary.Conv_IntToString` _array_index) " ; " (`KismetStringLibrary.Conv_NameToString` _itemid) " = " (`KismetStringLibrary.Conv_IntToString` _itemquantity)))))

(fn `SetFoodFazule`
  (params (Boolean :type Boolean))
  (if Boolean
    (bind _asbp_base_character (cast `/Game/Dialava/Blueprints/BP_BaseCharacter` (`GameplayStatics.GetPlayerCharacter` 0)))
    (set `/Game/Dialava/Blueprints/BP_BaseCharacter.CurrentFood` (+ (`/Game/Dialava/Blueprints/BP_BaseCharacter.CurrentFood` _asbp_base_character) 10.0) _asbp_base_character)))

(fn `SetFoodKapusta`
  (params (Boolean :type Boolean))
  (if Boolean
    (bind _asbp_base_character (cast `/Game/Dialava/Blueprints/BP_BaseCharacter` (`GameplayStatics.GetPlayerCharacter` 0)))
    (set `/Game/Dialava/Blueprints/BP_BaseCharacter.CurrentFood` (+ (`/Game/Dialava/Blueprints/BP_BaseCharacter.CurrentFood` _asbp_base_character) 20.0) _asbp_base_character)))

(fn `SetWaterVoda`
  (params (Boolean :type Boolean))
  (if Boolean
    (bind _asbp_base_character (cast `/Game/Dialava/Blueprints/BP_BaseCharacter` (`GameplayStatics.GetPlayerCharacter` 0)))
    (set `/Game/Dialava/Blueprints/BP_BaseCharacter.CurrentWater` (+ (`/Game/Dialava/Blueprints/BP_BaseCharacter.CurrentWater` _asbp_base_character) 20.0) _asbp_base_character)))

(fn `UseItem`
  (params (ItemID :type Name) (ItemQuantity :type Integer) (Index :type Integer))
  (bind _returnvalue (- ItemQuantity 1))
  (set `self.FlasaVody` (== ItemID "Flasa_Vody_001"))
  (set `self.KonzervaFazule` (== ItemID "Konzerva_Fazule_001"))
  (set `self.Kapusta` (== ItemID "Kapusta_001"))
  (if (or (`self.FlasaVody`) (`self.Kapusta`) (`self.KonzervaFazule`))
    (if (> _returnvalue 0)
      (`KismetArrayLibrary.Array_Set` (`self.ItemSlots`) (`local.Index`) (make `/Game/Dialava/Inventory/ItemData/S_ItemSlot` (`local.ItemID`) _returnvalue))
      (else
        (`KismetArrayLibrary.Array_Set` (`self.ItemSlots`) (`local.Index`) (make `/Game/Dialava/Inventory/ItemData/S_ItemSlot` "None"))))
    (`self.SetFoodKapusta` (`self.Kapusta`))
    (`self.SetFoodFazule` (`self.KonzervaFazule`))
    (`self.SetWaterVoda` (`self.FlasaVody`))
    (`self.UpdateInventory`)
    (`self.PlaySoundEffect` (`.Consume_9_E1C3DBEC440D24F1B87903BB62506FB9` (break `/Game/Dialava/Inventory/ItemData/S_ItemSoundEffects` (`self.GetItemSoundEffect` (`local.ItemID`)))))))